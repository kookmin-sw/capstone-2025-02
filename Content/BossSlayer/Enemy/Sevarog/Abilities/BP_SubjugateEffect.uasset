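; Short-lived effect actor for Sevarog's Subjugate ability that hits actors inside its collision box.
; On spawn it activates swirl and blast effects, then after a brief delay adds its owner to an ignore list and enables query-only collision.
; Overlapping actors join that list so each is processed once, and those implementing HitInterface receive GetHit.
; The actor destroys itself shortly after the collision window opens.
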(event OnComponentBeginOverlap(CollisionBox)
  (params (OverlappedComponent :type Primitive%20Component%20Object%20Reference) (OtherActor :type Actor%20Object%20Reference) (OtherComp :type Primitive%20Component%20Object%20Reference) (OtherBodyIndex :type Integer) (bFromSweep :type Boolean) (SweepResult :type Hit%20Result%20Structure%20%28by%20ref%29))
  (Utilities|IsValid OtherActor
    (:Is%20Valid
      (if (not (Utilities|Array|ContainsItem (Variables|Default|GetIgnoreActors) OtherActor))
        (Utilities|Array|AddUnique (Variables|Default|GetIgnoreActors) OtherActor)
        (if (Utilities|DoesObjectImplementInterface OtherActor "/Script/BossSlayer.HitInterface")
          (bind _ashit_interface (Utilities|Casting|CastToHitInterface OtherActor))
          (Class|HitInterface|GetHit _ashit_interface))))))

(event EventBeginPlay
  (Components|Activation|Activate (Variables|Default|GetSwirlFX) false)
  (Components|Activation|Activate (Variables|Default|GetBlastFX) false)
  (Utilities|FlowControl|Delay 0.3)
  (Utilities|Array|AddUnique (Variables|Default|GetIgnoreActors) (Components|GetOwner))
  (Collision|SetCollisionEnabled (Variables|Default|GetCollisionBox) "QueryOnly")
  (Utilities|FlowControl|Delay 1.5)
  (Actor|DestroyActor))

(event EventTick
  (params (DeltaSeconds :type Float%20%28single-precision%29)))

(fn ConstructionScript)