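; Sevarog enemy character for BossSlayer that equips a hammer on BeginPlay and provides two attacks through trigger events.
; Soul Siphon box-traces forward, then notifies non-invincible HitInterface targets and damages those that are BSCharacters.
; Subjugate spawns BP_Subjugate at the location of the AI controller's blackboard TargetActor.
; SetAttackMode passes the attack mode to the animation Blueprint.
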(event Custom|TriggerSubjugate
  (CallFunction|Subjugate))

(event Custom|TriggerSoulSiphon
  (CallFunction|SoulSiphon 4e+02))

(event EventBeginPlay
  (Class|Enemy|SpawnandEquipWeapon "HammerSocket"))

(event Collision|EventActorBeginOverlap
  (params (OtherActor :type Actor%20Object%20Reference)))

(event EventTick
  (params (DeltaSeconds :type Float%20%28single-precision%29)))

(fn ConstructionScript)

(fn SetAttackMode
  (params (NewParam :type E_AttackMode_Sevarog%20Enum :default "NewEnumerator0"))
  (bind _asabp_sevarog_enemy (Utilities|Casting|CastToABP_Sevarog_Enemy (Components|SkeletalMesh|GetAnimInstance (Variables|Character|GetMesh))))
  (Variables|/Game/BossSlayer/Enemy/Sevarog/ABP_Sevarog_Enemy.ABP_Sevarog_Enemy_C|SetAttackMode _asabp_sevarog_enemy NewParam))

(fn SoulSiphon
  (params (AttackRange :type Float%20%28double-precision%29))
  (LocalVariables|SetStart (Transformation|GetActorLocation))
  (bind _output_get (LocalVariables|SetEnd (+ (* (Transformation|GetActorForwardVector) AttackRange) (LocalVariables|GetStart))))
  (Utilities|Array|AddUnique (LocalVariables|GetActorsToIgnore) self)
  (bind (_outhit _returnvalue) (Collision|BoxTraceByChannel (LocalVariables|GetStart) _output_get "100.000000,100.000000,50.000000" (Math|Conversions|RotationFromXVector (Transformation|GetActorForwardVector)) "TraceTypeQuery1" false (LocalVariables|GetActorsToIgnore) "None"))
  (if _returnvalue
    (Utilities|IsValid (.HitActor (Collision|BreakHitResult _outhit))
      (:Is%20Valid
        (if (Utilities|DoesObjectImplementInterface (.HitActor (Collision|BreakHitResult _outhit)) "/Script/BossSlayer.HitInterface")
          (bind _ashit_interface (Utilities|Casting|CastToHitInterface (.HitActor (Collision|BreakHitResult _outhit))))
          (if (not (Class|HitInterface|GetbIsInvincible _ashit_interface))
            (Utilities|FlowControl|Sequence
              (:then_0
                (Class|HitInterface|GetHit _ashit_interface self))
              (:then_1
                (bind _asbscharacter (Utilities|Casting|CastToBSCharacter (.HitActor (Collision|BreakHitResult _outhit))))
                (Game|Damage|ApplyDamage _asbscharacter (Variables|Default|GetDamage) (AI|GetAIController self) self "/Script/Engine.DamageType")))))))))

(fn Subjugate
  (bind _self self)
  (bind _asaic_sevarog (Utilities|Casting|CastToAIC_Sevarog (Pawn|GetController)))
  (Utilities|IsValid (AI|Components|Blackboard|GetValueasObject (AI|GetBlackboard _asaic_sevarog) (Utilities|Name|MakeLiteralName "TargetActor"))
    (:Is%20Valid
      (bind _asactor (Utilities|Casting|CastToActor (AI|Components|Blackboard|GetValueasObject (AI|GetBlackboard _asaic_sevarog) (Utilities|Name|MakeLiteralName "TargetActor"))))
      (Game|SpawnActorfromClass "/Game/BossSlayer/Enemy/Sevarog/Abilities/BP_Subjugate.BP_Subjugate_C" (Math|Transform|MakeTransform (Transformation|GetActorLocation _asactor) "0, 0, 0" "1.000000,1.000000,1.000000") "AlwaysSpawn" "MultiplyWithRoot" _self _self)
      (return))))