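; BP_BlackKnight is the Black Knight boss character, which carries a mace.
; On BeginPlay it spawns BP_Mace and attaches it to the right-hand socket of its mesh.
; SetMoveSpeed maps the AI state to max walk speed, fastest in Chase and zero in Death.
; Attack is an empty event; unconnected montage chains would play jump or random attacks, then re-enable the blackboard CanAttack key.
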(event EventAttack
  (params (Distance :type Float%20%28double-precision%29)))

(event EventBeginPlay
  (bind _returnvalue (Game|SpawnActorfromClass "/Game/BossSlayer/Boss/Blueprints/BlackKnight/BP_Mace.BP_Mace_C" (Transformation|GetActorTransform) "Undefined" "MultiplyWithRoot" 0 0))
  (Transformation|AttachComponentToComponent _returnvalue (Variables|Character|GetMesh) "RightHandSocket" "SnapToTarget" "SnapToTarget" "SnapToTarget" true))

(event EventSetMoveSpeed
  (params (State :type E_Boss_State%20Enum :default "NewEnumerator0"))
  (Variables|/Script/Engine.CharacterMovementComponent|SetMaxWalkSpeed (Variables|Character|GetCharacterMovement) (Utilities|Select :Index State :NewEnumerator0 1e+02 :NewEnumerator1 1e+02 :NewEnumerator2 3.5e+02 :NewEnumerator3 1e+02 :NewEnumerator4 0.0)))

(fn ConstructionScript)