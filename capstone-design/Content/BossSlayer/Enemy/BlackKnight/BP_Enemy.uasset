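; BP_Enemy is the Black Knight enemy in BossSlayer, running a simple test behavior marked as being for animation testing.
; On BeginPlay it equips a weapon at the right-hand socket, then enters an endless delay-driven loop.
; Each cycle sends its AI controller toward the first BP_BSCharacter found, stops movement after a fixed delay, attacks, and pauses before repeating.
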(event EventBeginPlay
  ;[0.15 0.15 0.15 0.5] Animation 테스트용
  (Class|Enemy|SpawnandEquipWeapon "RightHandSocket")
  (bind _outactors (Actor|GetAllActorsOfClass "/Game/BossSlayer/BP_BSCharacter.BP_BSCharacter_C" :!label _label))
  (AI|Navigation|MovetoActor (AI|GetAIController self) (Utilities|Array|Get(acopy) _outactors) -1.0 true true true 0)
  (Utilities|FlowControl|Delay 5.0)
  (Components|Movement|StopMovementImmediately (Variables|Character|GetCharacterMovement))
  (Class|Enemy|Attack)
  (Utilities|FlowControl|Delay 2.0)
  (goto _label))

(event Collision|EventActorBeginOverlap
  (params (OtherActor :type Actor%20Object%20Reference)))

(event EventTick
  (params (DeltaSeconds :type Float%20%28single-precision%29)))

(fn ConstructionScript)